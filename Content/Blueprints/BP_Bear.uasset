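; Bear actor that roars and plays a melee attack animation when a ThirdPersonCharacter enters its trigger box.
; The box overlap spawns a 2D roar sound, then turns the Bear mesh on yaw only to face the character, with an offset for mesh orientation.
; After a fixed delay it returns to a looping idle animation; no damage is applied here.
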(event OnComponentBeginOverlap(Box)
  (params (OverlappedComponent :type Primitive%20Component%20Object%20Reference) (OtherActor :type Actor%20Object%20Reference) (OtherComp :type Primitive%20Component%20Object%20Reference) (OtherBodyIndex :type Integer) (bFromSweep :type Boolean) (SweepResult :type Hit%20Result%20Structure%20%28by%20ref%29))
  ;[1 1 1] Bear attack
  (bind _asthird_person_character (Utilities|Casting|CastToThirdPersonCharacter OtherActor))
  (bind _returnvalue (Audio|SpawnSound2D "/Game/Sounds/SW_BearRoar.SW_BearRoar"))
  (bind _output_get (Variables|Default|SetRoarReference _returnvalue))
  (Components|Activation|SetActive _output_get true false)
  (Transformation|SetWorldRotation (Variables|Default|GetBear) (Math|Rotator|MakeRotator 0.0 0.0 (+ (.Yaw (Math|Rotator|BreakRotator (Math|Rotator|FindLookatRotation (Transformation|GetWorldLocation (Variables|Default|GetBear)) (Transformation|GetActorLocation _asthird_person_character)))) -9e+01)) true false)
  (Components|Animation|PlayAnimation (Variables|Default|GetBear) "/Game/InfinityBladeAdversaries/Enemy/Enemy_Bear/Enemy_Bear_Animations/ExoGame_Bears_Attack_Melee.ExoGame_Bears_Attack_Melee" false)
  (Utilities|FlowControl|Delay 2.0)
  (Components|Animation|PlayAnimation (Variables|Default|GetBear) "/Game/InfinityBladeAdversaries/Enemy/Enemy_Bear/Enemy_Bear_Animations/ExoGame_Bears_Idle.ExoGame_Bears_Idle" true))

(event EventBeginPlay)

(event Collision|EventActorBeginOverlap
  (params (OtherActor :type Actor%20Object%20Reference)))

(event EventTick
  (params (DeltaSeconds :type Float%20%28single-precision%29)))

(fn ConstructionScript)